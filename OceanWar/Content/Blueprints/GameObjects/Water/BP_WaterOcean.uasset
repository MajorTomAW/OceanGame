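; Ocean water actor that sets up underwater, waterline and outline post-process effects within a box volume.
; Its construction script sizes the box to WaterSize and creates dynamic instances of the underwater and waterline materials.
; Both receive a water height from the actor's Z plus a small offset, then join the static outline material as weighted blendables on the post-process component.
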(fn `UserConstructionScript`
  (bind (_returnvalue_x _returnvalue_y _returnvalue_z) (`KismetMathLibrary.BreakVector` (`self.K2_GetActorLocation`)))
  (bind _returnvalue (+ _returnvalue_z 15.0))
  (`BoxComponent.SetBoxExtent` (`self.PostProcessSize`) (`self.WaterSize`) false)
  (`|ExecutionSequence`
    (:`then_0`
      (bind _returnvalue_2 (`KismetMaterialLibrary.CreateDynamicMaterialInstance` "/Game/Materials/Shading/PostProcessing/MI_PostProcess_Underwater.MI_PostProcess_Underwater"))
      (set `self.Underwater PP` _returnvalue_2)
      (bind _returnvalue_3 (`KismetMaterialLibrary.CreateDynamicMaterialInstance` "/Game/Materials/Shading/PostProcessing/MI_PostProcess_WaterLine.MI_PostProcess_WaterLine"))
      (set `self.WaterLine PP` _returnvalue_3))
    (:`then_1`
      (`self.Underwater PP`
        (:`then`
          (`MaterialInstanceDynamic.SetScalarParameterValue` (`self.Underwater PP`) "Water Height" _returnvalue))
        (:`else`)))
    (:`then_2`
      (`self.WaterLine PP`
        (:`then`
          (`|ExecutionSequence`
            (:`then_0`
              (`MaterialInstanceDynamic.SetScalarParameterValue` (`self.WaterLine PP`) "Water Height" _returnvalue))))
        (:`else`)))
    (:`then_4`
      (setmembers `PostProcessSettings` :`StructRef` (`PostProcessComponent.Settings` (`self.PostProcess`)) :`WeightedBlendables` (make `WeightedBlendables` (`|MakeArray` (make `WeightedBlendable` 1.0 (`self.WaterLine PP`)) (make `WeightedBlendable` 1.0 (`self.Underwater PP`)) (make `WeightedBlendable` 1.0 "/Game/Materials/Shading/PostProcessing/MI_PostProcess_Outline.MI_PostProcess_Outline") (make `WeightedBlendable` -1.0)))))))