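; Event-triggered gameplay ability that plays directional hit reactions when it receives an Ability.Event.HitReact event.
; It derives a yaw angle with atan2 from the reversed trace direction of the effect context's hit result, in world space without adjusting for actor rotation.
; That angle selects a Front, Right, Left or Back section of AM_Hull_HitReact, with Back split across the ±180 degree wrap.
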(event `self.K2_ActivateAbilityFromEvent`
  (params (EventData :type "GameplayEventData Structure (by ref)"))
  (bind (_bblockinghit _binitialoverlap _time _distance _location _impactpoint _normal _impactnormal _physmat _hitactor _hitcomponent _hitbonename _bonename _hititem _elementindex _faceindex _tracestart _traceend) (`GameplayStatics.BreakHitResult` (`AbilitySystemBlueprintLibrary.EffectContextGetHitResult` (`.ContextHandle` (break `GameplayEventData` (`self.CurrentEventData`))))))
  (bind (_returnvalue_x _returnvalue_y) (`KismetMathLibrary.BreakVector` (* (`KismetMathLibrary.GetDirectionUnitVector` _tracestart _traceend) -1.0)))
  (if (`BlueprintGameplayTagLibrary.MatchesTag` (`.EventTag` (break `GameplayEventData` EventData)) (struct :`TagName` "Ability.Event.HitReact") true)
    (set `self.HitDirection` (`KismetMathLibrary.DegAtan2` _returnvalue_y _returnvalue_x))
    (bind _returnvalue (`OceanityAbilityFunctionLibrary.GetMontageSectionBasedOnRangedFloat` (`self.HitDirection`) (`|MakeArray` (`OceanityAbilityFunctionLibrary.MakeRangedMontageSectionVector2D` "Front" (-45.0 45.0)) (`OceanityAbilityFunctionLibrary.MakeRangedMontageSectionVector2D` "Right" (45.0 135.0)) (`OceanityAbilityFunctionLibrary.MakeRangedMontageSectionVector2D` "Left" (-135.0 -45.0)) (`OceanityAbilityFunctionLibrary.MakeRangedMontageSectionVector2D` "Back" (135.0 180.0)) (`OceanityAbilityFunctionLibrary.MakeRangedMontageSectionVector2D` "Back" (-180.0 -135.0)))))
    (`AbilityTask_PlayMontageAndWait.CreatePlayMontageAndWaitProxy` "None" "/Game/Animations/Ship/Hull/Montages/AM_Hull_HitReact.AM_Hull_HitReact" 1.0 _returnvalue)))