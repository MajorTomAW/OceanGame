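; Event-triggered gameplay ability that grants coins to its owner on a Gameplay.Event.Hit.Success event.
; On an exact tag match and with authority, it builds a GE_Event_GiveCoins spec and applies it to its own ability system component.
; The event magnitude sets the coin amount as a SetByCaller value under Attribute.Meta.IncomingCoins.
; The graph never calls EndAbility.
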(event `self.K2_ActivateAbilityFromEvent`
  (params (EventData :type "GameplayEventData Structure (by ref)"))
  (bind _returnvalue (`self.GetAbilitySystemComponentFromActorInfo`))
  (if (`BlueprintGameplayTagLibrary.MatchesTag` (`.EventTag` (break `GameplayEventData` EventData)) (struct :`TagName` "Gameplay.Event.Hit.Success") true)
    (`self.K2_HasAuthority`
      (:`True`
        (bind _returnvalue_2 (`AbilitySystemBlueprintLibrary.AssignTagSetByCallerMagnitude` (`AbilitySystemComponent.MakeOutgoingSpec` _returnvalue "/Game/Blueprints/AbilitySystem/GameplayEffects/Event/GE_Event_GiveCoins.GE_Event_GiveCoins_C" 1.0 (`AbilitySystemComponent.MakeEffectContext` _returnvalue)) (struct :`TagName` "Attribute.Meta.IncomingCoins") (`.EventMagnitude` (break `GameplayEventData` (`self.CurrentEventData`)))))
        (`AbilitySystemComponent.BP_ApplyGameplayEffectSpecToSelf` (`self.GetAbilitySystemComponentFromActorInfo`) _returnvalue_2)))))